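; FreeCellCardArray is an actor that builds the grid of card sockets for a FreeCell card game.
; On BeginPlay it calls CreateRow repeatedly, spawning CardSocket actors tagged with their column index and collecting them in CardSockets.
; Socket transforms derive from the root's relative transform, with only Y varying by column, so successive rows spawn at the same positions.
; Each call also returns its row array, which BeginPlay leaves unused.
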(event `self.ReceiveBeginPlay`
  (for _ (range 25)
    (`self.CreateRow` 8)))

(fn `CreateRow`
  (params (NumberOfColumnsInRow :type Integer))
  (returns (Row :type "Array of /Game/Blueprints/Actors/CardSocket Object Reference"))
  (bind _returnvalue (`SceneComponent.GetRelativeTransform` (`self.DefaultSceneRoot`)))
  (set `self.tempRow` (`|MakeArray` null :!type "/Game/Blueprints/Actors/CardSocket Object Reference"))
  (for _index (range (+ NumberOfColumnsInRow 1))
    (bind _returnvalue_2 (`|SpawnActorFromClass` "/Game/Blueprints/Actors/CardSocket.CardSocket_C" (`KismetMathLibrary.MakeTransform` (`KismetMathLibrary.MakeVector` (.x (.location _returnvalue)) (* (- (.y (.location _returnvalue)) -13.0) (`KismetMathLibrary.Conv_IntToDouble` _index)) (.z (.location _returnvalue))) (.rotation _returnvalue) (.scale _returnvalue)) "Undefined" "OverrideRootScale" null null))
    (set `/Game/Blueprints/Actors/CardSocket.Column` _index _returnvalue_2)
    (`KismetArrayLibrary.Array_Add` (`self.tempRow`) _returnvalue_2)
    (`KismetArrayLibrary.Array_Add` (`self.CardSockets`) _returnvalue_2))
  (return (`self.tempRow`)))

(fn `UserConstructionScript`)