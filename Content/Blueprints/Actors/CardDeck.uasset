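; CardDeck is an actor that builds and shuffles a deck of playing cards when play begins.
; It nests loops over its Suits and Numbers arrays, spawning a Card actor at its root transform for each combination.
; Each card receives its suit and value, runs SetupCard and joins the Cards array, which is shuffled once the loops finish.
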(event `self.ReceiveBeginPlay`
  ;[1 1 1] Spawn 52 cards
  (for _array_element (`self.Suits`)
    (for _array_element_2 (`self.Numbers`)
      (bind _returnvalue (`|SpawnActorFromClass` "/Game/Blueprints/Actors/Card.Card_C" (`SceneComponent.K2_GetComponentToWorld` (`self.DefaultSceneRoot`)) "Undefined" "OverrideRootScale" null null))
      ;[1 1 1] Setup Card
      (set `/Game/Blueprints/Actors/Card.Suit` _array_element _returnvalue)
      (set `/Game/Blueprints/Actors/Card.Value` _array_element_2 _returnvalue)
      (`/Game/Blueprints/Actors/Card.SetupCard` _returnvalue)
      ;[1 1 1] Add Card to Deck
      (`KismetArrayLibrary.Array_Add` (`self.Cards`) _returnvalue)))
  ;[1 1 1] Shuffle Deck
  (`KismetArrayLibrary.Array_Shuffle` (`self.Cards`)))

(fn `UserConstructionScript`)